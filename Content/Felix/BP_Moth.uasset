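; BP_Moth is an interactable moth that shows dialogue from its MothText through a WG_Moth widget.
; Entering its box creates the widget and adds it to the viewport, and leaving removes it.
; Each Interact passes the text to the widget, reveals the text blocks and advances CurrentRow, removing the widget when no rows remain.
; A DoOnce gates Interact and is reset by ResetDialogue after each step.
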(event `self.Box.OnComponentBeginOverlap`
  (params (OverlappedComponent :type "PrimitiveComponent Object Reference") (OtherActor :type "Actor Object Reference") (OtherComp :type "PrimitiveComponent Object Reference") (OtherBodyIndex :type Integer) (bFromSweep :type Boolean) (SweepResult :type "HitResult Structure (by ref)"))
  (bind _returnvalue (`|CreateWidget` "/Game/Felix/WG_Moth.WG_Moth_C"))
  (bind _output_get (set `self.WG Moth` _returnvalue))
  (`UserWidget.AddToViewport` _output_get 0))

(event `self.Box.OnComponentEndOverlap`
  (params (OverlappedComponent :type "PrimitiveComponent Object Reference") (OtherActor :type "Actor Object Reference") (OtherComp :type "PrimitiveComponent Object Reference") (OtherBodyIndex :type Integer))
  (bind _wg_moth (`self.WG Moth`))
  (`/Engine/EditorBlueprintResources/StandardMacros.IsValid` _wg_moth
    (:`Is Valid`
      (`Widget.RemoveFromParent` _wg_moth))))

(event `/Game/ThirdPerson/Blueprints/I_Interact.Interact`
  (bind _wg_moth (`self.WG Moth`))
  (bind _wg_moth_2 (`self.WG Moth`))
  (bind _returnvalue (+ (`/Game/Felix/WG_Moth.currentRow` _wg_moth) 1))
  (`/Engine/EditorBlueprintResources/StandardMacros.DoOnce` false :!label _label
    (:`Completed`
      (set `/Game/Felix/WG_Moth.text` (`self.MothText`) _wg_moth)
      (`Widget.SetVisibility` (`/Game/Felix/WG_Moth.Textbox` _wg_moth) "Visible")
      (`Widget.SetVisibility` (`/Game/Felix/WG_Moth.TextBlock_0` _wg_moth) "Visible")
      (if (> _returnvalue (- (`KismetArrayLibrary.Array_Length` (`self.MothText`)) 1))
        (`Widget.RemoveFromParent` _wg_moth_2)
        (`self.ResetDialogue`)
        (else
          (set `/Game/Felix/WG_Moth.currentRow` _returnvalue _wg_moth_2)
          (`self.ResetDialogue`))))))

(event `ResetDialogue`
  (goto _label :!via `Reset`))

(fn `UserConstructionScript`)