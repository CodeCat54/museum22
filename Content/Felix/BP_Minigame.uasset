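; Interactable minigame Blueprint that, on Interact, moves the player's camera to its Arrow and, if the player's state allows, opens WG_Minigame and changes that state.
; MinigameNum selects one of six hardcoded sequences of increasing length, stored in the player character's MinigameArray.
; Each entry becomes a TableStruct pair of inverted value and sequence index, which is passed to the widget's StartMinigame.
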(event `/Game/ThirdPerson/Blueprints/I_Interact.Interact`
  (bind _tablestruct (`self.TableStruct`))
  ;[1 1 1] Construct minigame based on given variable
  (bind _asbp_third_person_character (cast `/Game/ThirdPerson/Blueprints/BP_ThirdPersonCharacter` (`GameplayStatics.GetPlayerCharacter` 0)))
  (`/Game/ThirdPerson/Blueprints/BP_ThirdPersonCharacter.ChangeCamera` _asbp_third_person_character (`self.Arrow`))
  (if (`|EnumEquality` (`/Game/ThirdPerson/Blueprints/BP_ThirdPersonCharacter.EPlayerState` _asbp_third_person_character) "NewEnumerator0")
    (bind _returnvalue (`|CreateWidget` "/Game/Felix/WG_Minigame.WG_Minigame_C"))
    (`UserWidget.AddToViewport` _returnvalue 0)
    (bind _asbp_third_person_character_2 (cast `/Game/ThirdPerson/Blueprints/BP_ThirdPersonCharacter` (`GameplayStatics.GetPlayerCharacter` 0)))
    (set `/Game/ThirdPerson/Blueprints/BP_ThirdPersonCharacter.EPlayerState` "NewEnumerator1" _asbp_third_person_character_2)
    (switch `int` (`self.MinigameNum`)
      (:`Default`
        ;[1 1 1] Different array per minigame
        (bind _output_get (set `/Game/ThirdPerson/Blueprints/BP_ThirdPersonCharacter.MinigameArray` (`|MakeArray` 1 4 4 1) _asbp_third_person_character_2 :!label _label)))
      (:`0`
        (goto _label))
      (:`1`
        (set `/Game/ThirdPerson/Blueprints/BP_ThirdPersonCharacter.MinigameArray` (`|MakeArray` 3 1 2 4 3) _asbp_third_person_character_2))
      (:`2`
        (set `/Game/ThirdPerson/Blueprints/BP_ThirdPersonCharacter.MinigameArray` (`|MakeArray` 2 2 1 2 4 3) _asbp_third_person_character_2))
      (:`3`
        (set `/Game/ThirdPerson/Blueprints/BP_ThirdPersonCharacter.MinigameArray` (`|MakeArray` 4 1 3 2 1 4 3) _asbp_third_person_character_2))
      (:`4`
        (set `/Game/ThirdPerson/Blueprints/BP_ThirdPersonCharacter.MinigameArray` (`|MakeArray` 4 4 3 4 2 1 2 4) _asbp_third_person_character_2))
      (:`5`
        (set `/Game/ThirdPerson/Blueprints/BP_ThirdPersonCharacter.MinigameArray` (`|MakeArray` 2 3 4 1 2 4 3 1 4) _asbp_third_person_character_2)))
    (`KismetArrayLibrary.Array_Clear` (`self.TableStruct`))
    (for (_array_element _array_index) _output_get
      (switch `int` (- _array_element 1)
        (:`0`
          (`KismetArrayLibrary.Array_Add` _tablestruct (make `/Game/Felix/S_NotesSrtucture` 3 _array_index)))
        (:`1`
          (`KismetArrayLibrary.Array_Add` _tablestruct (make `/Game/Felix/S_NotesSrtucture` 2 _array_index)))
        (:`2`
          (`KismetArrayLibrary.Array_Add` _tablestruct (make `/Game/Felix/S_NotesSrtucture` 1 _array_index)))
        (:`3`
          (`KismetArrayLibrary.Array_Add` _tablestruct (make `/Game/Felix/S_NotesSrtucture` 0 _array_index)))))
    (bind _foundwidgets (`WidgetBlueprintLibrary.GetAllWidgetsOfClass` "/Game/Felix/WG_Minigame.WG_Minigame_C"))
    (for _array_element_2 _foundwidgets
      (`/Game/Felix/WG_Minigame.StartMinigame` _array_element_2 _tablestruct))))

(fn `UserConstructionScript`)